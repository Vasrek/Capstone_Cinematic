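; BP_MyDummyPawn is a placeholder pawn that shows the main menu when play begins.
; On BeginPlay it creates WBP_MainMenu, adds it to the viewport, switches to UI-only input and shows the mouse cursor.
; Its PlayBTNClicked event calls CallStartTheGame, then restores game-only input and hides the cursor.
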(event `self.ReceiveBeginPlay`
  (bind _returnvalue (`GameplayStatics.GetPlayerController` 0))
  (bind _returnvalue_2 (`|CreateWidget` "/Game/Blueprint/Widgets/WBP_MainMenu.WBP_MainMenu_C"))
  (bind _output_get (set `self.MainMenuRef` _returnvalue_2))
  (`UserWidget.AddToViewport` _output_get 0)
  (`WidgetBlueprintLibrary.SetInputMode_UIOnlyEx` _returnvalue _output_get)
  (set `PlayerController.bShowMouseCursor` true _returnvalue))

(event `PlayBTNClicked`
  (bind _returnvalue (`GameplayStatics.GetPlayerController` 0))
  (`self.StartTheGame`)
  (`WidgetBlueprintLibrary.SetInputMode_GameOnly` _returnvalue)
  (set `PlayerController.bShowMouseCursor` false _returnvalue))

(fn `UserConstructionScript`)