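; Interactable door Blueprint that swings open once, to a yaw 90 degrees from its starting rotation.
; BeginPlay caches the start and target yaw; OpenDoor starts a looping timer on RotateDoor and clears CanBeUsed.
; RotateDoor eases the Door's world yaw with FInterpTo, zeroing pitch and roll, and clears the timer once the interpolated yaw nears the target.
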(event `self.ReceiveBeginPlay`
  (bind (_returnvalue_roll _returnvalue_pitch _returnvalue_yaw) (`KismetMathLibrary.BreakRotator` (`SceneComponent.K2_GetComponentRotation` (`self.Door`))))
  (bind _output_get (set `self.DefaultYaw` _returnvalue_yaw))
  (set `self.TargetYaw` (+ _output_get 90.0)))

(event `OpenDoor`
  (`KismetSystemLibrary.K2_SetTimer` null "RotateDoor" 0.01 true)
  (set `self.CanBeUsed?` false))

(fn `RotateDoor`
  (bind _door (`self.Door`))
  (bind _targetyaw (`self.TargetYaw`))
  (bind (_returnvalue_roll _returnvalue_pitch _returnvalue_yaw) (`KismetMathLibrary.BreakRotator` (`SceneComponent.K2_GetComponentRotation` _door)))
  (bind _returnvalue (`KismetMathLibrary.FInterpTo` _returnvalue_yaw _targetyaw (`GameplayStatics.GetWorldDeltaSeconds`) (`self.Interp Speed`)))
  (`SceneComponent.K2_SetWorldRotation` _door (`KismetMathLibrary.MakeRotator` 0.0 0.0 _returnvalue) false false)
  (if (`KismetMathLibrary.NearlyEqual_FloatFloat` _returnvalue _targetyaw 2.0)
    (`KismetSystemLibrary.K2_ClearTimer` null "RotateDoor")))

(fn `UserConstructionScript`
  (`parent.UserConstructionScript`))